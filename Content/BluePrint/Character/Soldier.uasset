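; Soldier is a selectable unit Blueprint for a turn-based strategy game, with a health bar, a fixed move range and an attack allowance.
; Each Tick it opens a W_Soldier widget once when clicked and clears the click when RTS_Cam selects something else.
; Tick also turns the W_Blood health bar toward the camera and restores AttackChance whenever PlayerTurn differs from the soldier's Camp.
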(event `self.ReceiveBeginPlay`
  (bind _asw_blood (cast `/Game/Widget/W_Blood` (`WidgetComponent.GetUserWidgetObject` (`self.HealthBar`))))
  (set `/Game/Widget/W_Blood.Owner` self _asw_blood))

(event `self.ReceiveTick`
  (params (DeltaSeconds :type "Float (single-precision)"))
  (bind _returnvalue (`GameplayStatics.GetPlayerPawn` 0))
  (bind _healthbar (`self.HealthBar`))
  (`|ExecutionSequence`
    (:`then_0`
      (`self.OpenWideget`))
    (:`then_1`
      (bind _asrts_cam (cast `/Game/BluePrint/RTS_Cam` _returnvalue))
      (if (not (== (`/Game/BluePrint/RTS_Cam.SelectionCha` _asrts_cam) self))
        (set `self.OnClick` false)))
    (:`then_2`
      (bind _asrts_cam_2 (cast `/Game/BluePrint/RTS_Cam` (`GameplayStatics.GetPlayerPawn` 0)))
      (`SceneComponent.K2_SetWorldRotation` _healthbar (`KismetMathLibrary.FindLookAtRotation` (`SceneComponent.K2_GetComponentLocation` _healthbar) (`SceneComponent.K2_GetComponentLocation` (`/Game/BluePrint/RTS_Cam.RTSCam` _asrts_cam_2))) false false))
    (:`then_3`
      (bind _asrts_cam_3 (cast `/Game/BluePrint/RTS_Cam` _returnvalue))
      (if (!= (`/Game/BluePrint/RTS_Cam.PlayerTurn` _asrts_cam_3) (`self.Camp`))
        (set `self.AttackChance` 1)))))

(event `OpenWideget`
  (if (`self.OnClick`)
    (if (not (`self.OpenWidget`))
      (bind _returnvalue (`|CreateWidget` "/Game/Widget/W_Soldier.W_Soldier_C" (`GameplayStatics.GetPlayerController` 0)))
      (set `/Game/Widget/W_Soldier.Owner` self _returnvalue)
      (`UserWidget.AddToViewport` _returnvalue 0)
      (`WidgetBlueprintLibrary.SetInputMode_GameAndUIEx` (`GameplayStatics.GetPlayerController` 0) _returnvalue)
      (set `self.OpenWidget` true))))

(fn `UserConstructionScript`
  (`parent.UserConstructionScript`)
  (set `self.MoveableDistance` 510.0))