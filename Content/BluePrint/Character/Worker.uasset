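; Worker unit for a turn-based RTS that carries a briefcase and builds bastions and houses.
; Tick opens a W_Worker widget when clicked and turns OperationForParent codes into spawned buildings, paid from RTS_Cam resources.
; IsAction blocks repeat builds and resets, with MovementChance, when the turn is not its camp's.
; Tick also turns the health bar toward the camera and handles death with a montage and destroy.
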(event `self.ReceiveBeginPlay`
  (bind _asw_character_blood (cast `/Game/Widget/W_CharacterBlood` (`WidgetComponent.GetUserWidgetObject` (`self.HealthBar`))))
  (set `/Game/Widget/W_CharacterBlood.Owner` self _asw_character_blood)
  (bind _returnvalue (`|SpawnActorFromClass` "/Game/BluePrint/BP_Briefcase.BP_Briefcase_C" (`KismetMathLibrary.MakeTransform` (0.0 0.0 0.0)) "Undefined" "OverrideRootScale" null null))
  (`self.K2_AttachToComponent` _returnvalue (`self.Mesh`) "Briefcase" "SnapToTarget" "KeepRelative" "KeepRelative" true))

(event `self.ReceiveTick`
  (params (DeltaSeconds :type "Float (single-precision)"))
  (`|ExecutionSequence`
    (:`then_0`
      (if (`self.OnClick`)
        (if (not (`self.OpenW`))
          (bind _returnvalue (`|CreateWidget` "/Game/Widget/W_Worker.W_Worker_C" (`GameplayStatics.GetPlayerController` 0)))
          (`UserWidget.AddToViewport` _returnvalue 0)
          (set `/Game/Widget/W_Worker.Owner` self _returnvalue)
          (set `self.OpenW` true)
          (`WidgetBlueprintLibrary.SetInputMode_GameAndUIEx` (`GameplayStatics.GetPlayerController` 0) _returnvalue))))
    (:`then_1`
      (bind _asrts_cam (cast `/Game/BluePrint/RTS_Cam` (`GameplayStatics.GetPlayerPawn` 0)))
      (if (not (== (`/Game/BluePrint/RTS_Cam.SelectionCha` _asrts_cam) self))
        (set `self.OnClick` false)))
    (:`then_2`
      (if (== (`self.OperationForParent`) 2)
        (if (`self.IsAction`)
          (`KismetSystemLibrary.PrintString` "This unit have been do the operation" :!label _label)
          (set `self.OperationForParent` 0)
          (else
            (bind _wood (`/Game/BluePrint/RTS_Cam.Wood` _asrts_cam))
            (bind _iron (`/Game/BluePrint/RTS_Cam.Iron` _asrts_cam))
            (if (and (>= _wood 100.0) (>= _iron 50.0))
              (bind _returnvalue_2 (`|SpawnActorFromClass` "/Game/BluePrint/BP_Bastion.BP_Bastion_C" (`KismetMathLibrary.MakeTransform` (`self.SelectionLocation`)) "Undefined" "OverrideRootScale" null null))
              (set `/Game/BluePrint/RTS_Cam.Wood` (- _wood 100.0) _asrts_cam)
              (set `/Game/BluePrint/RTS_Cam.Iron` (- _iron 50.0) _asrts_cam)
              (set `self.OperationForParent` 0)
              (set `self.IsAction` true)
              (set `/Game/BluePrint/BP_BUilding.Camp` (`self.Camp`) _returnvalue_2)
              (set `/Game/BluePrint/BP_BUilding.isTraining` true _returnvalue_2))))))
    (:`then_3`
      (`self.BloodFactToCamera`)
      (bind _asrts_cam_2 (cast `/Game/BluePrint/RTS_Cam` (`GameplayStatics.GetPlayerPawn` 0)))
      (if (!= (`/Game/BluePrint/RTS_Cam.PlayerTurn` _asrts_cam_2) (`self.Camp`))
        (set `self.IsAction` false)
        (set `self.MovementChance` true)))
    (:`then_4`
      (if (== (`self.OperationForParent`) 3)
        (if (`self.IsAction`)
          (goto _label)
          (else
            (bind _coal (`/Game/BluePrint/RTS_Cam.Coal` _asrts_cam))
            (bind _wood_2 (`/Game/BluePrint/RTS_Cam.Wood` _asrts_cam))
            (if (and (>= _coal 50.0) (>= _wood_2 100.0))
              (bind _returnvalue_3 (`|SpawnActorFromClass` "/Game/BluePrint/BP_House.BP_House_C" (`KismetMathLibrary.MakeTransform` (`self.SelectionLocation`)) "Undefined" "OverrideRootScale" null null))
              (set `/Game/BluePrint/RTS_Cam.Coal` (- _coal 50.0) _asrts_cam)
              (set `/Game/BluePrint/RTS_Cam.Wood` (- _wood_2 100.0) _asrts_cam)
              (set `self.OperationForParent` 0)
              (set `self.IsAction` true)
              (set `/Game/BluePrint/BP_BUilding.Camp` (`self.Camp`) _returnvalue_3)
              (set `/Game/BluePrint/BP_BUilding.isTraining` true _returnvalue_3))))))
    (:`then_5`
      (if (<= (`self.Health`) 0.0)
        (`/Engine/EditorBlueprintResources/StandardMacros.DoOnce` false
          (:`Completed`
            (`SkeletalMeshComponent.PlayAnimation` (`self.Mesh`) "/Game/Mannequin/Animations/Death_1_Montage.Death_1_Montage" false)
            (`KismetSystemLibrary.Delay` 1.8)
            (`self.K2_DestroyActor` (stale `self.ReceiveBeginPlay` _returnvalue))
            (`self.K2_DestroyActor`)))))))

(event `BloodFactToCamera`
  (bind _healthbar (`self.HealthBar`))
  ;[1 1 1] HP Bar face to player
  (bind _asrts_cam (cast `/Game/BluePrint/RTS_Cam` (`GameplayStatics.GetPlayerPawn` 0)))
  (`SceneComponent.K2_SetWorldRotation` _healthbar (`KismetMathLibrary.FindLookAtRotation` (`SceneComponent.K2_GetComponentLocation` _healthbar) (`SceneComponent.K2_GetComponentLocation` (`/Game/BluePrint/RTS_Cam.RTSCam` _asrts_cam))) false false))

(fn `UserConstructionScript`
  (`parent.UserConstructionScript`)
  (set `self.MoveableDistance` 330.0))