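; AIEnemies is an AI-controlled character for a turn-based RTS-camera game, with health, a team camp and a once-per-turn movement chance.
; On BeginPlay it links itself to its W_CharacterBlood health bar widget, which Tick rotates to face the RTS camera.
; Tick also restores MovementChance whenever the player turn differs from its Camp.
; Move requests pass to BP_AIController, and GetDamage subtracts from Health.
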(event `self.ReceiveBeginPlay`
  (bind _asw_character_blood (cast `/Game/Widget/W_CharacterBlood` (`WidgetComponent.GetUserWidgetObject` (`self.HealthBar`))))
  (set `/Game/Widget/W_CharacterBlood.Owner` self _asw_character_blood))

(event `self.ReceiveTick`
  (params (DeltaSeconds :type "Float (single-precision)"))
  (`|ExecutionSequence`
    (:`then_0`
      (`self.HPFaceTo`))
    (:`then_1`
      (bind _asrts_cam (cast `/Game/BluePrint/RTS_Cam` (`GameplayStatics.GetPlayerPawn` 0)))
      (if (!= (`/Game/BluePrint/RTS_Cam.PlayerTurn` _asrts_cam) (`self.Camp`))
        (set `self.MovementChance` true)))))

(event `/Game/BluePrint/Character/BP_Interface.MoveCharacterTo`
  (params (Location :type "Vector Structure"))
  (bind _asbp_aicontroller (cast `/Game/BluePrint/Character/BP_AIController` (`self.GetController`)))
  (message `/Game/BluePrint/Character/BP_Interface.MoveCharacterTo` _asbp_aicontroller Location))

(event `Get Damage`
  (params (damage :type "Float (double-precision)"))
  (set `self.Health` (- (`self.Health`) damage)))

(event `HPFaceTo`
  (bind _healthbar (`self.HealthBar`))
  (bind _asrts_cam (cast `/Game/BluePrint/RTS_Cam` (`GameplayStatics.GetPlayerPawn` 0)))
  (`SceneComponent.K2_SetWorldRotation` _healthbar (`KismetMathLibrary.FindLookAtRotation` (`SceneComponent.K2_GetComponentLocation` _healthbar) (`SceneComponent.K2_GetComponentLocation` (`/Game/BluePrint/RTS_Cam.RTSCam` _asrts_cam))) false false))

(fn `UserConstructionScript`)