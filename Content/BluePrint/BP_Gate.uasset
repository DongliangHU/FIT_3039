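; BP_Gate is a camp-owned gate building in a turn-based RTS whose destruction ends the match.
; BeginPlay links the gate to its durability bar widget.
; Tick shows an end menu tagged with the gate's camp while durability is depleted, clears training outside that camp's turn, and calls FaceToPlayer and DurabiltyGoToZero.
; Tick also applies an alternate material once for camp 1.
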(event `self.ReceiveBeginPlay`
  (bind _asw_building_durability (cast `/Game/Widget/W_BuildingDurability` (`WidgetComponent.GetUserWidgetObject` (`self.DurabilityBar`))))
  (set `/Game/Widget/W_BuildingDurability.Owner` self _asw_building_durability))

(event `self.ReceiveTick`
  (params (DeltaSeconds :type "Float (single-precision)"))
  (`|ExecutionSequence`
    (:`then_0`
      (if (<= (`self.Durability`) 0.0)
        (bind _returnvalue (`|CreateWidget` "/Game/Widget/EndMenu.EndMenu_C"))
        (`UserWidget.AddToViewport` _returnvalue 0)
        (set `/Game/Widget/EndMenu.Camp` (`self.Camp`) _returnvalue)))
    (:`then_1`
      (bind _asrts_cam (cast `/Game/BluePrint/RTS_Cam` (`GameplayStatics.GetPlayerPawn` 0)))
      (if (!= (`/Game/BluePrint/RTS_Cam.PlayerTurn` _asrts_cam) (`self.Camp`))
        (set `self.isTraining` false)))
    (:`then_2`
      (`self.face to Player`))
    (:`then_3`
      (`self.DurabiltyGoToZero`))
    (:`then_4`
      (`/Engine/EditorBlueprintResources/StandardMacros.DoOnce` false
        (:`Completed`
          (if (== (`self.Camp`) 1)
            (`PrimitiveComponent.SetMaterial` (`self.StaticMesh`) 0 "/Game/Material/M_Gate_Inst.M_Gate_Inst")))))))

(fn `UserConstructionScript`)