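; BP_Gold is a gold pickup actor that adds a fixed amount of gold to the player's RTS_Cam pawn when gathered.
; Tick polls the Gather flag, and once it is set, casts the player pawn, increments its Gold, prints a message and destroys the actor.
; The construction script stores the actor's starting location, which is not read in this graph.
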(event `self.ReceiveBeginPlay`)

(event `self.ReceiveTick`
  (params (DeltaSeconds :type "Float (single-precision)"))
  (if (`self.Gather`)
    (bind _asrts_cam (cast `/Game/BluePrint/RTS_Cam` (`GameplayStatics.GetPlayerPawn` 0)))
    (set `/Game/BluePrint/RTS_Cam.Gold` (+ (`/Game/BluePrint/RTS_Cam.Gold` _asrts_cam) 100.0) _asrts_cam)
    (`KismetSystemLibrary.PrintString` "Gathering 100 Gold")
    (`self.K2_DestroyActor`)))

(fn `UserConstructionScript`
  (set `self.origanlLocation` (`self.K2_GetActorLocation`)))