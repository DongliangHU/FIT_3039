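; BP_Grid is a grid tile that highlights itself as selectable for the character or building selected in the RTS game.
; Each Tick, while unoccupied, it reads the RTS_Cam pawn and switches material based on whether its distance from the selected location falls within a ring.
; Cursor hover over a selectable tile shows the selection material.
; Overlaps on the Avaliable component mark the tile occupied and clear its highlight.
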(event `self.ReceiveTick`
  (params (DeltaSeconds :type "Float (single-precision)"))
  (if (not (`self.IsSometingOnIt`))
    (`self.ShowAvaliable`)
    (`self.ShowBuildingAvailiable`)))

(event `self.ReceiveActorBeginCursorOver`
  (if (`self.IsSometingOnIt`)
    _
    (elif (`self.IsOn`)
      (`PrimitiveComponent.SetMaterial` (`self.StaticMesh`) 0 "/Game/Material/Grid_Selection.Grid_Selection")
      (set `self.isRed` true))))

(event `self.ReceiveActorEndCursorOver`
  (set `self.isRed` false)
  (if (`self.IsOn`)
    (`PrimitiveComponent.SetMaterial` (`self.StaticMesh`) 0 "/Game/Material/Grid_CanSelection.Grid_CanSelection")
    (else
      (`PrimitiveComponent.SetMaterial` (`self.StaticMesh`) 0 "/Game/Material/Grid_normal.Grid_normal"))))

(event `ShowAvaliable`
  (bind _staticmesh (`self.StaticMesh`))
  ;[1 1 1] Show Which plaform can select
  (bind _asrts_cam (cast `/Game/BluePrint/RTS_Cam` (`GameplayStatics.GetPlayerPawn` 0)))
  (if (`/Game/BluePrint/RTS_Cam.SelectCharacterOrNot` _asrts_cam)
    (bind _returnvalue (`KismetMathLibrary.Vector_Distance` (`self.K2_GetActorLocation`) (`/Game/BluePrint/RTS_Cam.ControlLocation` _asrts_cam)))
    (if (and (< _returnvalue (`/Game/BluePrint/RTS_Cam.RecordMovableDis` _asrts_cam)) (> _returnvalue 150.0))
      (if (not (`self.isRed`))
        (`PrimitiveComponent.SetMaterial` _staticmesh 0 "/Game/Material/Grid_CanSelection.Grid_CanSelection")
        (set `self.IsOn` true))
      (else
        (`PrimitiveComponent.SetMaterial` _staticmesh 0 "/Game/Material/Grid_normal.Grid_normal")
        (set `self.IsOn` false)))))

(event `self.Avaliable.OnComponentBeginOverlap`
  (params (OverlappedComponent :type "PrimitiveComponent Object Reference") (OtherActor :type "Actor Object Reference") (OtherComp :type "PrimitiveComponent Object Reference") (OtherBodyIndex :type Integer) (bFromSweep :type Boolean) (SweepResult :type "HitResult Structure (by ref)"))
  (set `self.IsSometingOnIt` true)
  (set `self.IsOn` false)
  (`PrimitiveComponent.SetMaterial` (`self.StaticMesh`) 0 "/Game/Material/Grid_normal.Grid_normal"))

(event `self.Avaliable.OnComponentEndOverlap`
  (params (OverlappedComponent :type "PrimitiveComponent Object Reference") (OtherActor :type "Actor Object Reference") (OtherComp :type "PrimitiveComponent Object Reference") (OtherBodyIndex :type Integer))
  (set `self.IsSometingOnIt` false)
  (set `self.IsOn` true))

(event `ShowBuildingAvailiable`
  (bind _staticmesh (`self.StaticMesh`))
  (bind _asrts_cam (cast `/Game/BluePrint/RTS_Cam` (`GameplayStatics.GetPlayerPawn` 0)))
  (if (`/Game/BluePrint/RTS_Cam.SelectBuildingOrNot` _asrts_cam)
    (bind _returnvalue (`KismetMathLibrary.Vector_Distance` (`self.K2_GetActorLocation`) (`/Game/BluePrint/RTS_Cam.BulidingLocation` _asrts_cam)))
    (if (and (< _returnvalue 330.0) (> _returnvalue 150.0))
      (if (not (`self.isRed`))
        (`PrimitiveComponent.SetMaterial` _staticmesh 0 "/Game/Material/Grid_CanSelection.Grid_CanSelection")
        (set `self.IsOn` true))
      (else
        (`PrimitiveComponent.SetMaterial` _staticmesh 0 "/Game/Material/Grid_normal.Grid_normal")
        (set `self.IsOn` false)))))

(fn `UserConstructionScript`)