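; RTS camera pawn that handles player input for a two-player, turn-based grid strategy game.
; Axis, wheel and right-drag input pan, zoom and rotate the view.
; Left-click selects own-camp units or any building; cursor traces on right-click resolve moves, construction, gathering, attacks and resource-paid troop training, according to operation state and per-turn action flags.
; Turn events possess the PlayerOne or PlayerTwo pawn and set its PlayerTurn.
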(event `self.ReceiveBeginPlay`)

(event `InputAxis|MoveForward`
  (params (AxisValue :type "Float (single-precision)"))
  ;[1 1 1] basic movement
  (`self.K2_AddActorLocalOffset` (`KismetMathLibrary.MakeVector` (* AxisValue (`self.MoveSpeed`)))))

(event `InputAxis|MoveRight`
  (params (AxisValue :type "Float (single-precision)"))
  ;[1 1 1] basic movement
  (`self.K2_AddActorLocalOffset` (`KismetMathLibrary.MakeVector` 0.0 (* AxisValue (`self.MoveSpeed`)))))

(event `Key|MouseScrollUp`
  (params (Key :type "Key Structure"))
  (bind _springarm (`self.SpringArm`))
  ;[1 1 1] Wheel to view closely or far away
  (:`Pressed`
    (set `SpringArmComponent.TargetArmLength` (- (`SpringArmComponent.TargetArmLength` _springarm) 50.0) _springarm)))

(event `Key|MouseScrollDown`
  (params (Key :type "Key Structure"))
  (bind _springarm (`self.SpringArm`))
  ;[1 1 1] Wheel to view closely or far away
  (:`Pressed`
    (set `SpringArmComponent.TargetArmLength` (+ (`SpringArmComponent.TargetArmLength` _springarm) 50.0) _springarm)))

(event `InputAxisKey|MouseX`
  (params (AxisValue :type "Float (single-precision)"))
  ;[1 1 1] Right click to routate view sight
  (`/Engine/EditorBlueprintResources/StandardMacros.Gate` true :!label _label
    (:`Exit`
      (`self.K2_AddActorLocalRotation` (`KismetMathLibrary.MakeRotator` 0.0 0.0 (* AxisValue (`self.RotateSpeed`)))))))

(event `Key|RightMouseButton`
  (params (Key :type "Key Structure"))
  (bind _returnvalue (`GameplayStatics.GetPlayerController` 0))
  ;[1 1 1] Right click to routate view sight
  (:`Pressed`
    (set `PlayerController.bShowMouseCursor` false _returnvalue)
    (`|ExecutionSequence`
      (:`then_0`
        (goto _label :!via `Open`))
      (:`then_1`
        (goto _label_2 :!via `Open`))))
  (:`Released`
    (set `PlayerController.bShowMouseCursor` true _returnvalue)
    (`|ExecutionSequence`
      (:`then_0`
        (goto _label :!via `Close`))
      (:`then_1`
        (goto _label_2 :!via `Close`)))))

(event `InputAxisKey|MouseY`
  (params (AxisValue :type "Float (single-precision)"))
  ;[1 1 1] Right click to routate view sight
  (`/Engine/EditorBlueprintResources/StandardMacros.Gate` true :!label _label_2
    (:`Exit`
      (`SceneComponent.K2_AddLocalRotation` (`self.RTSCam`) (`KismetMathLibrary.MakeRotator` 0.0 (* AxisValue (`self.RotateSpeed`))) false false))))

(event `self.ReceiveTick`
  (params (DeltaSeconds :type "Float (single-precision)"))
  (`|ExecutionSequence`
    (:`then_0`
      (if (`self.SelectCharacterOrNot`)
        (set `self.ControlLocation` (`self.K2_GetActorLocation` (stale `Key|LeftMouseButton` _asaienemies)))
        (else
          (set `self.ControlLocation` (10000000.0 0.0 10000.0)))))
    (:`then_1`
      (switch `int` (`self.BuildingOperation`)
        (:`0`
          (set `self.BulidingLocation` (0.0 0.0 10000.0)))
        (:`1`
          (set `self.BulidingLocation` (`self.K2_GetActorLocation` (`self.SelectionBuilding`)) :!label _label_3))
        (:`2`
          (goto _label_3))
        (:`3`
          (goto _label_3))))))

(event `Key|LeftMouseButton`
  (params (Key :type "Key Structure"))
  (:`Pressed`
    (bind _asaienemies (cast `/Game/BluePrint/Character/AIEnemies` (`.HitActor` (`GameplayStatics.BreakHitResult` (`PlayerController.GetHitResultUnderCursorByChannel` (`GameplayStatics.GetPlayerController` 0) "TraceTypeQuery1" true))))
      (:`then`
        (set `self.OperationNum` 0)
        ;[1 1 1] Left click to select the character, right click to move the specific location
        (if (== (`/Game/BluePrint/Character/AIEnemies.Camp` _asaienemies) (`self.PlayerTurn`))
          (`|ExecutionSequence`
            (:`then_0`
              (goto _label_5 :!via `Open`))
            (:`then_1`
              (set `self.SelectionCha` _asaienemies))
            (:`then_2`
              (set `self.SelectCharacterOrNot` true)
              (set `/Game/BluePrint/Character/AIEnemies.OnClick` true _asaienemies))
            (:`then_3`
              (set `self.RecordMovableDis` (`/Game/BluePrint/Character/AIEnemies.MoveableDistance` _asaienemies))))
          (else
            (`KismetSystemLibrary.PrintString` "select  your camp")
            (set `self.SelectCharacterOrNot` false :!label _label_4)
            (set `self.SelectionCha` null)
            (set `self.RecordMovableDis` 0.0)
            (goto _label_5 :!via `Close`))))
      (:`CastFailed`
        (goto _label_4)))))

(event `Key|RightMouseButton`
  (params (Key :type "Key Structure"))
  (:`Pressed`
    (bind _asbp_grid (cast `/Game/BluePrint/BP_Grid` (`.HitActor` (`GameplayStatics.BreakHitResult` (`PlayerController.GetHitResultUnderCursorByChannel` (`GameplayStatics.GetPlayerController` 0) "TraceTypeQuery1" true)))))
    (switch `int` (`self.OperationNum`)
      (:`0`
        ;[1 1 1] Left click to select the character, right click to move the specific location
        (`/Engine/EditorBlueprintResources/StandardMacros.Gate` true :!label _label_5
          (:`Exit`
            (if (`/Game/BluePrint/BP_Grid.IsOn` _asbp_grid)
              (if (`/Game/BluePrint/BP_Grid.IsSometingOnIt` _asbp_grid)
                _
                (elif (`/Game/BluePrint/Character/AIEnemies.MovementChance` (stale `Key|LeftMouseButton` _asaienemies))
                  (if (`self.SelectCharacterOrNot`)
                    (bind _returnvalue (`self.K2_GetActorLocation` _asbp_grid))
                    (message `/Game/BluePrint/Character/BP_Interface.MoveCharacterTo` (stale `Key|LeftMouseButton` _asaienemies) _returnvalue)
                    (set `/Game/BluePrint/Character/AIEnemies.MovementChance` false (stale `Key|LeftMouseButton` _asaienemies)))
                  (else
                    (`KismetSystemLibrary.PrintString` "This Unit Has been move in this turn"))))))))
      (:`1`
        (set `/Game/BluePrint/Character/AIEnemies.OperationForParent` 1 (stale `Key|LeftMouseButton` _asaienemies))
        (set `self.OperationNum` 0))
      (:`2`
        ;[1 1 1] Spawn building
        (set `self.OperationNum` 0)
        (if (`/Game/BluePrint/BP_Grid.IsOn` _asbp_grid)
          (set `/Game/BluePrint/Character/AIEnemies.OperationForParent` 2 (stale `Key|LeftMouseButton` _asaienemies))
          (set `/Game/BluePrint/Character/AIEnemies.SelectionLocation` _returnvalue (stale `Key|LeftMouseButton` _asaienemies))))
      (:`3`
        (set `self.OperationNum` 0)
        (if (`/Game/BluePrint/BP_Grid.IsOn` _asbp_grid)
          (set `/Game/BluePrint/Character/AIEnemies.OperationForParent` 3 (stale `Key|LeftMouseButton` _asaienemies))
          (set `/Game/BluePrint/Character/AIEnemies.SelectionLocation` _returnvalue (stale `Key|LeftMouseButton` _asaienemies)))))))

(event `Key|RightMouseButton`
  (params (Key :type "Key Structure"))
  ;[1 1 1] Worker Gather the resource
  (:`Pressed`
    (bind _asworker (cast `/Game/BluePrint/Character/Worker` (`self.SelectionCha`)))
    (bind _asbp_resource (cast `/Game/BluePrint/BP_Resource` (`.HitActor` (`GameplayStatics.BreakHitResult` (`PlayerController.GetHitResultUnderCursorByChannel` (`GameplayStatics.GetPlayerController` 0) "TraceTypeQuery1" true)))))
    (if (`/Game/BluePrint/Character/Worker.IsAction` _asworker)
      (`KismetSystemLibrary.PrintString` "This unit have been do the operation")
      (elif (<= (`KismetMathLibrary.Vector_Distance` (`self.K2_GetActorLocation` _asbp_resource) (`self.K2_GetActorLocation` _asworker)) (`self.RecordMovableDis`))
        (set `/Game/BluePrint/BP_Resource.Gather` true _asbp_resource)
        (set `/Game/BluePrint/Character/Worker.IsAction` true _asworker)))))

(event `Key|LeftMouseButton`
  (params (Key :type "Key Structure"))
  (bind (_bblockinghit _binitialoverlap _time _distance _location _impactpoint _normal _impactnormal _physmat _hitactor) (`GameplayStatics.BreakHitResult` (`PlayerController.GetHitResultUnderCursorByChannel` (`GameplayStatics.GetPlayerController` 0) "TraceTypeQuery1" true)))
  ;[1 1 1] Selecting the building
  (:`Pressed`
    (bind _asbp_building (cast `/Game/BluePrint/BP_BUilding` _hitactor)
      (:`then`
        (set `/Game/BluePrint/BP_BUilding.OnClick` true _asbp_building)
        (set `self.SelectionBuilding` _hitactor)
        (set `self.SelectBuildingOrNot` true))
      (:`CastFailed`
        (set `self.SelectionBuilding` null)
        (set `self.SelectBuildingOrNot` false)))))

(event `Key|RightMouseButton`
  (params (Key :type "Key Structure"))
  (bind _selectionbuilding (`self.SelectionBuilding`))
  (bind _buildingoperation (`self.BuildingOperation`))
  (bind _playerturn (`self.PlayerTurn`))
  (bind _returnvalue (`self.K2_GetActorLocation` (`.HitActor` (`GameplayStatics.BreakHitResult` (`PlayerController.GetHitResultUnderCursorByChannel` (`GameplayStatics.GetPlayerController` 0) "TraceTypeQuery1" true)))))
  ;[1 1 1] Bastion Create the troop
  (:`Pressed`
    (`|ExecutionSequence`
      (:`then_0`
        (bind _asbp_bastion (cast `/Game/BluePrint/BP_Bastion` _selectionbuilding))
        (if (`/Game/BluePrint/BP_BUilding.isTraining` _asbp_bastion)
          (`KismetSystemLibrary.PrintString` "This unit has been action" :!label _label_6)
          (else
            (set `/Game/BluePrint/BP_BUilding.isTraining` true _asbp_bastion)
            (switch `int` _buildingoperation
              (:`1`
                (if (and (>= (`self.Gold`) 100.0) (>= (`self.Iron`) 100.0))
                  (bind _returnvalue_2 (`AIBlueprintHelperLibrary.SpawnAIFromClass` "/Game/BluePrint/Character/Soldier.Soldier_C" null _returnvalue (struct) false null))
                  (set `self.Gold` (- (`self.Gold`) 100.0))
                  (set `self.Iron` (- (`self.Iron`) 100.0))
                  (bind _assoldier (cast `/Game/BluePrint/Character/Soldier` _returnvalue_2))
                  (set `/Game/BluePrint/Character/AIEnemies.Camp` (`self.PlayerTurn`) _assoldier)
                  (set `/Game/BluePrint/Character/AIEnemies.MovementChance` false _assoldier)
                  (set `/Game/BluePrint/Character/Soldier.AttackChance` 0 _assoldier)
                  (set `self.BuildingOperation` 0 :!label _label_7)))
              (:`2`
                (if (and (>= (`self.Gold`) 150.0) (>= (`self.Iron`) 50.0) (>= (`self.Coal`) 50.0) (>= (`self.Wood`) 50.0))
                  (bind _returnvalue_3 (`AIBlueprintHelperLibrary.SpawnAIFromClass` "/Game/BluePrint/Character/Cannon.Cannon_C" null _returnvalue (struct) false null))
                  (set `self.Gold` (- (`self.Gold`) 150.0))
                  (set `self.Iron` (- (`self.Iron`) 50.0))
                  (set `self.Coal` (- (`self.Coal`) 50.0))
                  (set `self.Wood` (- (`self.Wood`) 50.0))
                  (bind _ascannon (cast `/Game/BluePrint/Character/Cannon` _returnvalue_3))
                  (set `/Game/BluePrint/Character/AIEnemies.Camp` _playerturn _ascannon)
                  (set `/Game/BluePrint/Character/AIEnemies.MovementChance` false _ascannon)
                  (set `/Game/BluePrint/Character/Cannon.AttackChance` 0 _ascannon)
                  (goto _label_7)))))))
      (:`then_1`
        (bind _asbp_house (cast `/Game/BluePrint/BP_House` _selectionbuilding))
        (if (`/Game/BluePrint/BP_BUilding.isTraining` _asbp_house)
          (goto _label_6)
          (else
            (set `/Game/BluePrint/BP_BUilding.isTraining` true _asbp_house)
            (if (== _buildingoperation 3)
              (if (and (>= (`self.Gold`) 50.0) (>= (`self.Coal`) 100.0))
                (bind _returnvalue_4 (`AIBlueprintHelperLibrary.SpawnAIFromClass` "/Game/BluePrint/Character/Worker.Worker_C" null _returnvalue (struct) false null))
                (set `self.Gold` (- (`self.Gold`) 50.0))
                (set `self.Coal` (- (`self.Coal`) 100.0))
                (bind _asworker (cast `/Game/BluePrint/Character/Worker` _returnvalue_4))
                (set `/Game/BluePrint/Character/AIEnemies.Camp` _playerturn _asworker)
                (set `/Game/BluePrint/Character/AIEnemies.MovementChance` false _asworker)
                (set `/Game/BluePrint/Character/Worker.IsAction` true _asworker)
                (goto _label_7)))))))))

(event `Key|RightMouseButton`
  (params (Key :type "Key Structure"))
  (bind _selectioncha (`self.SelectionCha`))
  (bind _selectioncha_2 (`self.SelectionCha`))
  (bind (_bblockinghit _binitialoverlap _time _distance _location _impactpoint _normal _impactnormal _physmat _hitactor) (`GameplayStatics.BreakHitResult` (`PlayerController.GetHitResultUnderCursorByChannel` (`GameplayStatics.GetPlayerController` 0) "TraceTypeQuery1" true)))
  ;[1 1 1] Attack
  (:`Pressed`
    (`|ExecutionSequence`
      (:`then_0`
        (bind _asaienemies (cast `/Game/BluePrint/Character/AIEnemies` _hitactor))
        (if (== (`self.OperationNum`) 1)
          (`|ExecutionSequence`
            (:`then_0`
              (bind _assoldier (cast `/Game/BluePrint/Character/Soldier` _selectioncha_2))
              (if (== (`/Game/BluePrint/Character/Soldier.AttackChance` _assoldier) 1)
                (bind _camp (`/Game/BluePrint/Character/AIEnemies.Camp` _asaienemies))
                (if (== (`/Game/BluePrint/Character/AIEnemies.Camp` _assoldier) _camp)
                  (`KismetSystemLibrary.PrintString` "Same Camp" :!label _label_8)
                  (elif (<= (`KismetMathLibrary.Vector_Distance` (`self.K2_GetActorLocation` _assoldier) (`self.K2_GetActorLocation` _asaienemies)) (`self.RecordMovableDis`))
                    (`/Game/BluePrint/Character/AIEnemies.Get Damage` _asaienemies 0.0)
                    (set `/Game/BluePrint/Character/Soldier.AttackChance` 0 _assoldier)
                    (else
                      (`KismetSystemLibrary.PrintString` "Out of attack range" :!label _label_9))))
                (else
                  (`KismetSystemLibrary.PrintString` "Have been attack" :!label _label_10))))
            (:`then_1`
              (bind _ascannon (cast `/Game/BluePrint/Character/Cannon` _selectioncha_2))
              (if (== (`/Game/BluePrint/Character/Cannon.AttackChance` _ascannon) 1)
                (if (== (`/Game/BluePrint/Character/AIEnemies.Camp` _ascannon) _camp)
                  (goto _label_8)
                  (else
                    (bind _returnvalue (`self.K2_GetActorLocation` _asaienemies))
                    (if (<= (`KismetMathLibrary.Vector_Distance` (`self.K2_GetActorLocation` _ascannon) _returnvalue) (`self.RecordMovableDis`))
                      (`/Game/BluePrint/Character/AIEnemies.Get Damage` _asaienemies 0.0)
                      (set `/Game/BluePrint/Character/Cannon.AttackChance` 0 _ascannon)
                      (else
                        (goto _label_9)))))
                (else
                  (goto _label_10)))))))
      (:`then_1`
        (bind _asbp_building (cast `/Game/BluePrint/BP_BUilding` _hitactor))
        (if (== (`self.OperationNum`) 1)
          (`|ExecutionSequence`
            (:`then_0`
              (bind _assoldier_2 (cast `/Game/BluePrint/Character/Soldier` _selectioncha))
              (if (== (`/Game/BluePrint/Character/Soldier.AttackChance` _assoldier_2) 1)
                (bind _camp_2 (`/Game/BluePrint/BP_BUilding.Camp` _asbp_building))
                (if (== (`/Game/BluePrint/Character/AIEnemies.Camp` _assoldier_2) _camp_2)
                  (goto _label_8)
                  (elif (<= (`KismetMathLibrary.Vector_Distance` _returnvalue (`self.K2_GetActorLocation` _assoldier_2)) (`self.RecordMovableDis`))
                    (`/Game/BluePrint/BP_BUilding.DecreaseDurability` _asbp_building)
                    (set `/Game/BluePrint/Character/Soldier.AttackChance` 0 _assoldier_2)
                    (else
                      (goto _label_9))))
                (else
                  (goto _label_10))))
            (:`then_1`
              (bind _ascannon_2 (cast `/Game/BluePrint/Character/Cannon` _selectioncha))
              (if (== (`/Game/BluePrint/Character/Cannon.AttackChance` _ascannon_2) 1)
                (if (== (`/Game/BluePrint/Character/AIEnemies.Camp` _ascannon_2) _camp_2)
                  (goto _label_8)
                  (elif (<= (`KismetMathLibrary.Vector_Distance` (`self.K2_GetActorLocation`) (`self.K2_GetActorLocation`)) (`self.RecordMovableDis`))
                    (`/Game/BluePrint/BP_BUilding.DecreaseDurability` _asbp_building)
                    (set `/Game/BluePrint/Character/Cannon.AttackChance` 0 _ascannon_2)
                    (else
                      (goto _label_9))))
                (else
                  (goto _label_10))))))))))

(event `PlayerOneTurn`
  ;[1 1 1] Change Player
  (bind _outactors (`GameplayStatics.GetAllActorsOfClass` "/Game/BluePrint/PlayerOne.PlayerOne_C"))
  (bind _output (`|GetArrayItem` _outactors))
  (`Controller.Possess` (`GameplayStatics.GetPlayerController` 0) _output)
  (set `/Game/BluePrint/RTS_Cam.PlayerTurn` 1 _output))

(event `PlayerTwoTurn`
  ;[1 1 1] Change Player
  (bind _outactors (`GameplayStatics.GetAllActorsOfClass` "/Game/BluePrint/PlayerTwo.PlayerTwo_C"))
  (bind _output (`|GetArrayItem` _outactors))
  (`Controller.Possess` (`GameplayStatics.GetPlayerController` 0) _output)
  (set `/Game/BluePrint/RTS_Cam.PlayerTurn` 2 _output))

(fn `UserConstructionScript`)