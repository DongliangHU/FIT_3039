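; BP_House is a selectable building that belongs to a camp and has a durability bar and a house UI widget.
; BeginPlay links the durability widget to itself, and a click flag opens W_House once while OpenWidget is unset.
; Tick polls RTS_Cam to clear the click flag when deselected and IsTraining outside its camp's turn.
; Tick also runs player-facing and zero-durability routines, and a one-time material swap for camp 1.
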(event `self.ReceiveBeginPlay`
  (bind _asw_building_durability (cast `/Game/Widget/W_BuildingDurability` (`WidgetComponent.GetUserWidgetObject` (`self.DurabilityBar`))))
  (set `/Game/Widget/W_BuildingDurability.Owner` self _asw_building_durability))

(event `self.ReceiveTick`
  (params (DeltaSeconds :type "Float (single-precision)"))
  (bind _returnvalue (`GameplayStatics.GetPlayerPawn` 0))
  (`|ExecutionSequence`
    (:`then_0`
      (`self.OpenHouseWidget`))
    (:`then_1`
      (bind _asrts_cam (cast `/Game/BluePrint/RTS_Cam` _returnvalue))
      (if (not (== (`/Game/BluePrint/RTS_Cam.SelectionBuilding` _asrts_cam) self))
        (set `self.OnClick` false)))
    (:`then_2`
      (bind _asrts_cam_2 (cast `/Game/BluePrint/RTS_Cam` _returnvalue))
      (if (!= (`/Game/BluePrint/RTS_Cam.PlayerTurn` _asrts_cam_2) (`self.Camp`))
        (set `self.isTraining` false)))
    (:`then_3`
      (`self.face to Player`))
    (:`then_4`
      (`self.DurabiltyGoToZero`))
    (:`then_5`
      (`/Engine/EditorBlueprintResources/StandardMacros.DoOnce` false
        (:`Completed`
          (if (== (`self.Camp`) 1)
            (`PrimitiveComponent.SetMaterial` (`self.StaticMesh`) 0 "/Game/Material/M_House_Inst.M_House_Inst")))))))

(event `OpenHouseWidget`
  ;[1 1 1] Open the widget
  (if (`self.OnClick`)
    (if (not (`self.OpenWidget`))
      (bind _returnvalue (`|CreateWidget` "/Game/Widget/W_House.W_House_C"))
      (`UserWidget.AddToViewport` _returnvalue 0)
      (set `self.OpenWidget` true)
      (`WidgetBlueprintLibrary.SetInputMode_GameAndUIEx` (`GameplayStatics.GetPlayerController` 0) _returnvalue)
      (set `/Game/Widget/W_House.Owner` self _returnvalue))))

(fn `UserConstructionScript`)